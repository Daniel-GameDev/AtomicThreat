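; BP_LauncherBase_GridElement is the base grid element for launchers that fire rockets at target coordinates.
; LaunchRocket spawns the requested rocket class at the LaunchPoint with a fixed rotation, passing in the target, assigning the owning player and increasing its default parameters.
; Rockets implementing BPI_MultiRocket also receive an array of targets through an interface message.
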(event Custom|LaunchRocket
  (params (RocketType :type BP%20Rocket%20Base%20Class%20Reference) (IncreaseValue :type Float%20%28single-precision%29) (TargetCoordinate :type Vector) (TargetsArray :type Array%20of%20Vectors) (Player :type BP%20Atomic%20Player%20Controller%20Object%20Reference))
  (bind _returnvalue (Game|SpawnActorfromClass RocketType (Math|Transform|MakeTransform (Transformation|GetWorldLocation (Variables|Default|GetLaunchPoint)) "90.000000, 0, 0" "1,1,1") "Undefined" 0 TargetCoordinate 0))
  (Variables|/Game/AtomicThreat/Blueprints/Gameplay/Rockets/BP_RocketBase.BP_RocketBase_C|SetRocketPlayerController _returnvalue Player)
  (Default|IncreaseDefaultRocketParams _returnvalue IncreaseValue)
  (if (Utilities|DoesObjectImplementInterface _returnvalue "/Game/AtomicThreat/Blueprints/Common/BPI_MultiRocket.BPI_MultiRocket_C")
    (Class|BPIMultiRocket|SetTargetsArray(Message) _returnvalue TargetsArray)))

(event EventBeginPlay
  (|CallParentFunction) ; This node is disabled and will not be called.\nDrag off pins to build functionality.
)

(event Collision|EventActorBeginOverlap
  (params (OtherActor :type Actor%20Object%20Reference))
  (|CallParentFunction OtherActor) ; This node is disabled and will not be called.\nDrag off pins to build functionality.
)

(event EventTick
  (params (DeltaSeconds :type Float%20%28single-precision%29))
  (|CallParentFunction DeltaSeconds) ; This node is disabled and will not be called.\nDrag off pins to build functionality.
)

(fn ConstructionScript
  (|CallParentFunction))