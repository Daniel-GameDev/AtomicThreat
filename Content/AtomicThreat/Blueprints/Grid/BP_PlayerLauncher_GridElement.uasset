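; Player-controlled rocket launcher grid element that spawns and possesses the player's atomic pawn on BeginPlay.
; It also spawns an attached ammo actor, repositioned to a default display location on X and Z.
; Rocket launches first call UseAmmo, printing "Empty" when it returns true and otherwise deferring to the parent's launch logic.
; Any overlap on the capsule destroys both the ammo actor and the launcher.
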(event OnComponentBeginOverlap(Capsule)
  (params (OverlappedComponent :type Primitive%20Component%20Object%20Reference) (OtherActor :type Actor%20Object%20Reference) (OtherComp :type Primitive%20Component%20Object%20Reference) (OtherBodyIndex :type Integer) (bFromSweep :type Boolean) (SweepResult :type Hit%20Result%20Structure%20%28by%20ref%29))
  (Actor|DestroyActor (Variables|Default|GetAmmo))
  (Actor|DestroyActor))

(event EventBeginPlay
  (bind _defaultdisplaylocation (Variables|Default|GetDefaultDisplayLocation))
  (|CallParentFunction)
  (bind _returnvalue (Game|SpawnActorfromClass "/Game/AtomicThreat/Blueprints/Framework/BP_AtomicPawn.BP_AtomicPawn_C" (Transformation|GetActorTransform) "Undefined" 0 self 0))
  (Pawn|Possess (Game|GetPlayerController 0) _returnvalue)
  (bind _returnvalue_2 (Game|SpawnActorfromClass "/Game/AtomicThreat/Blueprints/Gameplay/BP_Ammo.BP_Ammo_C" (Math|Transform|MakeTransform (Transformation|GetActorLocation) "0, 0, 0" "1,1,1") "Undefined" 0 0))
  (bind _output_get (Variables|Default|SetAmmo _returnvalue_2))
  (Transformation|AttachActorToActor _output_get self "None" "KeepWorld" "KeepRelative" "KeepRelative" false)
  (Transformation|SetWorldLocation (Variables|/Script/Engine.Actor|GetRootComponent (Variables|Default|GetAmmo)) (Math|Vector|MakeVector (.x _defaultdisplaylocation) (.y (Transformation|GetWorldLocation (Variables|/Script/Engine.Actor|GetRootComponent (Variables|Default|GetAmmo)))) (.z _defaultdisplaylocation)) false false))

(event Collision|EventActorBeginOverlap
  (params (OtherActor :type Actor%20Object%20Reference))
  (|CallParentFunction OtherActor) ; This node is disabled and will not be called.\nDrag off pins to build functionality.
)

(event EventTick
  (params (DeltaSeconds :type Float%20%28single-precision%29))
  (|CallParentFunction DeltaSeconds) ; This node is disabled and will not be called.\nDrag off pins to build functionality.
)

(event EventLaunchRocket
  (params (RocketType :type BP%20Rocket%20Base%20Class%20Reference) (IncreaseValue :type Float%20%28single-precision%29) (TargetCoordinate :type Vector :default "0, 0, 0") (TargetsArray :type Array%20of%20Vectors) (Player :type BP%20Atomic%20Player%20Controller%20Object%20Reference))
  (bind _empty (Default|UseAmmo (Variables|Default|GetAmmo)))
  (if _empty
    (Development|PrintString "Empty")
    (else
      (|CallParentFunction RocketType IncreaseValue TargetCoordinate TargetsArray Player))))

(fn ConstructionScript
  (|CallParentFunction))