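; BP_LauncherBase_GridElement is a base Blueprint for rocket launcher elements on the grid.
; Its LaunchRocket event spawns an actor of the configurable RocketType class at the LaunchPoint component's world location with a fixed rotation.
; The target coordinate is passed into the rocket at spawn, and the launcher itself runs no other gameplay logic.
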(event Custom|LaunchRocket
  (params (TargetCoordinate :type Vector))
  (Game|SpawnActorfromClass (Variables|Default|GetRocketType) (Math|Transform|MakeTransform (Transformation|GetWorldLocation (Variables|Default|GetLaunchPoint)) "90.000000, 0, 0" "1,1,1") "Undefined" 0 TargetCoordinate 0))

(event EventBeginPlay
  (|CallParentFunction) ; This node is disabled and will not be called.\nDrag off pins to build functionality.
)

(event Collision|EventActorBeginOverlap
  (params (OtherActor :type Actor%20Object%20Reference))
  (|CallParentFunction OtherActor) ; This node is disabled and will not be called.\nDrag off pins to build functionality.
)

(event EventTick
  (params (DeltaSeconds :type Float%20%28single-precision%29))
  (|CallParentFunction DeltaSeconds) ; This node is disabled and will not be called.\nDrag off pins to build functionality.
)

(fn ConstructionScript
  (|CallParentFunction))