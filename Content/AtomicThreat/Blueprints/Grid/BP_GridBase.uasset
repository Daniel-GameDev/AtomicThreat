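; BP_GridBase is a grid actor that lays out element actors in a single row along Y at a set spacing.
; Its construction script can add debug meshes along that row and fill the default class list.
; CreateGrid2 spawns, attaches and indexes actors from a passed or default list, falling back to defaults for invalid classes.
; ClearGrid2 destroys attached actors, while the CreateGrid and ClearGrid events are empty stubs.
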(event Custom|CreateGrid
  ;[1 1 1] Delete at end
)

(event Custom|ClearGrid)

(fn ConstructionScript
  (Utilities|FlowControl|Sequence
    (:then_0
      (if (Variables|Debug|GetbShowDebugGrid)
        (CallFunction|CreateGridHiddeninGame)))
    (:then_1
      (if (Variables|Default|GetUseDefault)
        (for _index (range 0 (Variables|Debug|GetGridSizeIndexForDefaultAndDebug))
          (Utilities|Array|Add (Variables|Default|GetDefaultGridElements) (Variables|Default|GetDefaultGridElement)))))))

(fn CreateGridHiddeninGame
  (for _index (range 0 (Variables|Debug|GetGridSizeIndexForDefaultAndDebug))
    (bind _returnvalue (AddComponent|AddStaticMeshComponent false (Math|Transform|MakeTransform (select (== _index 0) (LocalVariables|GetLocal_RelativeLoc) (Math|Vector|MakeVector (.X (Math|Vector|BreakVector (LocalVariables|GetLocal_RelativeLoc))) (+ (.Y (Math|Vector|BreakVector (LocalVariables|GetLocal_RelativeLoc))) (Variables|Default|GetGridSpacing)) (.Z (Math|Vector|BreakVector (LocalVariables|GetLocal_RelativeLoc))))) "0, 0, 0" "1,1,1")))
    (LocalVariables|SetLocal_RelativeLoc (Variables|/Script/Engine.SceneComponent|GetRelativeLocation _returnvalue))
    (Components|StaticMesh|SetStaticMesh _returnvalue (Variables|Debug|GetDebugGridMesh))
    (Development|SetHiddeninGame _returnvalue false false)))

(fn CreateGrid2
  (params (UseDefaultGrid :type Boolean) (Grid :type Array%20of%20BP%20Grid%20Element%20Base%20Class%20References))
  (if UseDefaultGrid
    (LocalVariables|SetLocal_GridElements (Variables|Default|GetDefaultGridElements))
    (else
      (LocalVariables|SetLocal_GridElements Grid)))
  (for (_array_element _array_index) (LocalVariables|GetLocal_GridElements)
    (if (Utilities|IsValidClass _array_element)
      (LocalVariables|SetLocal_SpawnClass _array_element)
      (else
        (LocalVariables|SetLocal_SpawnClass (Utilities|Array|Get(acopy) (Variables|Default|GetDefaultGridElements) _array_index))))
    (bind _returnvalue (Game|SpawnActorfromClass (LocalVariables|GetLocal_SpawnClass) (Math|Transform|MakeTransform (select (== _array_index 0) (Variables|Default|GetActorLocation) (Math|Vector|MakeVector (.X (Math|Vector|BreakVector (Variables|Default|GetActorLocation))) (+ (.Y (Math|Vector|BreakVector (Variables|Default|GetActorLocation))) (Variables|Default|GetGridSpacing)) (.Z (Math|Vector|BreakVector (Variables|Default|GetActorLocation))))) "0, 0, 0" "1,1,1") "Undefined" 0 0))
    (Variables|Default|SetActorLocation (Transformation|GetActorLocation _returnvalue))
    (Transformation|AttachActorToActor _returnvalue self "None" "KeepRelative" "KeepRelative" "KeepRelative" false)
    (Variables|/Game/AtomicThreat/Blueprints/Grid/GridElements/BP_GridElementBase.BP_GridElementBase_C|SetIndex _returnvalue _array_index)
    (Utilities|Array|Add (LocalVariables|GetLocal_GridElementsRef) _returnvalue))
  (Variables|Default|SetActorLocation "0, 0, 0")
  (return (LocalVariables|GetLocal_GridElementsRef)))

(fn ClearGrid2
  (bind _output_get (LocalVariables|SetNewLocalVar_0 (Actor|GetAttachedActors true)))
  (for (_array_element _array_index) _output_get
    (Actor|DestroyActor _array_element)
    (Development|PrintString (Utilities|String|ToString(Integer) _array_index)))
  (Development|PrintString "Hello"))