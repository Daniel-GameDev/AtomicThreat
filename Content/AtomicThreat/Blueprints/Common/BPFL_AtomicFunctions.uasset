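; Blueprint function library for Atomic Threat with shared helpers for round difficulty and rocket-count notifications.
; GetDifficultyDataFunction maps a round index to a difficulty data table row, returning the summed rocket count, difficulty increment and rocket type array.
; RocketNotifyFunction forwards a notify type and local rocket count to the game mode through BPI_RocketsLeft, if implemented.
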(fn GetDifficultyDataFunction
  (params (Round :type Integer))
  (bind _outrownames (DataTable|GetDataTableRowNames (LocalVariables|GetDifficultyDataTable)))
  (bind _output_get (LocalVariables|SetDataTableRowNames _outrownames))
  (bind _returnvalue (Utilities|GetDataTableRow (LocalVariables|GetDifficultyDataTable) (Utilities|Array|Get(acopy) _output_get Round))
    (:then
      (for _array_element (.RocketTypes (Utilities|Struct|BreakSDifficultyLevelValues _returnvalue))
        (LocalVariables|SetLocal_RocketsNum (+ (.Num (Utilities|Struct|BreakSRockets _array_element)) (LocalVariables|GetLocal_RocketsNum))))
      (return (LocalVariables|GetLocal_RocketsNum) (.DifficultyIncrement (Utilities|Struct|BreakSDifficultyLevelValues _returnvalue)) (.RocketTypes (Utilities|Struct|BreakSDifficultyLevelValues _returnvalue))))))

(fn RocketNotifyFunction
  (params (RocketsNum :type Integer) (NotifyType :type ENotify%20Enum :default "NewEnumerator0"))
  (bind _returnvalue (Game|GetGameMode))
  (if (Utilities|DoesObjectImplementInterface _returnvalue "/Game/AtomicThreat/Blueprints/Common/BPI_RocketsLeft.BPI_RocketsLeft_C")
    (if (== RocketsNum 0)
      (Class|BPIRocketsLeft|NotifyGameModeRockets(Message) _returnvalue (LocalVariables|GetLocal_Rockets) NotifyType)
      (else
        (Class|BPIRocketsLeft|NotifyGameModeRockets(Message) _returnvalue (LocalVariables|GetLocal_Rockets) NotifyType)))))