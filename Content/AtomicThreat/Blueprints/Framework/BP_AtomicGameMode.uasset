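; BP_AtomicGameMode is the game mode for AtomicThreat, tracking rounds in which city elements and rockets decide the outcome.
; StartRound builds the city grid, counts its attached actors and starts the spawn manager.
; Destroyed elements decrement toward a printed loss, while rocket notifications adjust a count that prints "NEXT ROUND" at zero.
; NextRound is empty, and GetPoints reads player state and pawn points through BPI_Points without using the result.
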(event Custom|NextRound)

(event Custom|GetPoints
  (bind _returnvalue (Game|GetPlayerController 0))
  (bind _returnvalue_2 (Pawn|GetControlledPawn _returnvalue))
  (bind _playerstate (Variables|/Script/Engine.Controller|GetPlayerState _returnvalue))
  (if (Utilities|DoesObjectImplementInterface _playerstate "/Game/AtomicThreat/Blueprints/Common/BPI_Points.BPI_Points_C")
    (bind _points (Class|BPIPoints|GetPoints(Message) _playerstate))
    (if (Utilities|DoesObjectImplementInterface _returnvalue_2 "/Game/AtomicThreat/Blueprints/Common/BPI_Points.BPI_Points_C")
      (bind _points_2 (Class|BPIPoints|GetPoints(Message) _returnvalue_2)))))

(event Custom|OnCityElementDestroyed
  (params (DestroyedActor :type Actor%20Object%20Reference))
  (bind _result (Math|Integer|DecrementInt (Variables|Default|GetCityElementOnLevel))
    (:%20%20
      (if (== _result 0)
        (Development|PrintString "GAME LOST!" true true "(R=1.000000,G=0.000000,B=0.009501,A=1.000000)" 5.0)))))

(event Custom|StartRound
  (Default|CreateGrid (Variables|Default|GetCityGrid))
  (Variables|Default|SetCityElementOnLevel (Utilities|Array|Length (Actor|GetAttachedActors (Variables|Default|GetCityGrid) true)))
  (Default|SpawnerStartRound (Variables|Default|GetSpawnManager)))

(event Custom|RocketsLeftCheck
  (if (== (Variables|Default|GetRockets%20Num) 0)
    (Development|PrintString "NEXT ROUND" true true "(R=1.000000,G=0.000000,B=0.009501,A=1.000000)" 5.0)))

(event EventNotifyGameModeRockets
  (params (RocketsNum :type Integer) (NotifyType :type ENotify%20Enum :default "NewEnumerator0"))
  (switch Utilities|FlowControl|Switch|SwitchonENotify NotifyType
    (:NewEnumerator0
      (Variables|Default|SetRockets%20Num (+ RocketsNum (Variables|Default|GetRockets%20Num))))
    (:NewEnumerator1
      (Variables|Default|SetRockets%20Num (- (Variables|Default|GetRockets%20Num) RocketsNum))))
  (CallFunction|RocketsLeftCheck))

(fn ConstructionScript)