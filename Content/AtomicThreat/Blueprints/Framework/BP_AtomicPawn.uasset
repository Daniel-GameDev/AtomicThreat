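; BP_AtomicPawn is the player pawn that fires defensive rockets from a launcher at the point under the mouse cursor.
; Pressing Launch traces under the cursor and, on a hit, tells its Launcher to fire a single defence rocket at that location on behalf of the player controller.
; It also reports the launcher's remaining rocket count, which GetPoints returns as the pawn's points.
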(event EventBeginPlay)

(event Collision|EventActorBeginOverlap
  (params (OtherActor :type Actor%20Object%20Reference)))

(event Input|ActionEvents|InputActionLaunch
  (params (Key :type Key%20Structure :default "None"))
  (bind _returnvalue (Game|GetPlayerController 0))
  (bind (_hitresult _returnvalue_2) (Game|Player|GetHitResultUnderCursorbyChannel _returnvalue "TraceTypeQuery3" true))
  (:Pressed
    (if _returnvalue_2
      (if (Utilities|IsValid (Variables|Default|GetLauncher))
        (Default|LaunchRocket (Variables|Default|GetLauncher) "/Game/AtomicThreat/Blueprints/Gameplay/BP_SingleRocket_Defence.BP_SingleRocket_Defence_C" 0.0 (.Location (Collision|BreakHitResult _hitresult)) (Utilities|Array|MakeArray "0, 0, 0") (.AsBP%20Atomic%20Player%20Controller (Utilities|Casting|CastToBP_AtomicPlayerController (Game|GetPlayerController 0))))))))

(fn ConstructionScript)

(fn GetLauncherAmmoLeft
  (bind _launcher (Variables|Default|GetLauncher))
  (if (Utilities|IsValid _launcher)
    (return (Utilities|Array|Length (Variables|/Game/AtomicThreat/Blueprints/Gameplay/BP_Ammo.BP_Ammo_C|GetRockets (Variables|/Game/AtomicThreat/Blueprints/Grid/BP_PlayerLauncher_GridElement.BP_PlayerLauncher_GridElement_C|GetAmmo _launcher))))
    (else
      (return 0))))

(fn GetPoints
  (return (CallFunction|GetLauncherAmmoLeft)))