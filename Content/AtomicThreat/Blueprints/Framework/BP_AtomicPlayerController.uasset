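; Player controller for the Atomic Threat game that owns and manages the UI widgets for the start, round, next-round and game-lost screens.
; On BeginPlay it shows the cursor, adds the temporary start screen and registers itself with the BP_AtomicPlayerState.
; Events create or remove screens and push points, bonus, round and rocket values into the round widget.
; Game-lost widget creation is marked unfinished.
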(event EventBeginPlay
  (Variables|Default|SetbShowMouseCursor true)
  (bind _returnvalue (UserInterface|CreateWidget "/Game/AtomicThreat/Blueprints/UI/WBP_TempStart.WBP_TempStart_C"))
  (UserInterface|Viewport|AddtoViewport _returnvalue 0)
  (bind _asbp_atomic_player_state (Utilities|Casting|CastToBP_AtomicPlayerState (Variables|GetPlayerState)))
  (Variables|/Game/AtomicThreat/Blueprints/Framework/BP_AtomicPlayerState.BP_AtomicPlayerState_C|SetCurrentAtomicPlayer _asbp_atomic_player_state self))

(event EventUpdatedGameRoundBonus
  (params (Bonus :type Integer))
  (Variables|/Game/AtomicThreat/Blueprints/UI/WBP_GameRound.WBP_GameRound_C|SetBonus (Variables|Default|GetGameRoundWidget) Bonus))

(event EventUpdatedGameRoundNum
  (params (Round :type Integer))
  (Variables|/Game/AtomicThreat/Blueprints/UI/WBP_GameRound.WBP_GameRound_C|SetRound (Variables|Default|GetGameRoundWidget) Round))

(event EventUpdatedGameRoundRockets
  (params (Rockets :type Integer))
  (Variables|/Game/AtomicThreat/Blueprints/UI/WBP_GameRound.WBP_GameRound_C|SetRockets (Variables|Default|GetGameRoundWidget) Rockets))

(event EventCreateGameRoundWidget
  (bind _returnvalue (UserInterface|CreateWidget "/Game/AtomicThreat/Blueprints/UI/WBP_GameRound.WBP_GameRound_C"))
  (bind _output_get (Variables|Default|SetGameRoundWidget _returnvalue))
  (UserInterface|Viewport|AddtoViewport _output_get 0))

(event EventCreateGameLostWidget
  ;[1 1 1] Unfinished
  (bind _returnvalue (UserInterface|CreateWidget "/Game/AtomicThreat/Blueprints/UI/WBP_GameLost.WBP_GameLost_C"))
  (bind _output_get (Variables|Default|SetGameLostWidget _returnvalue))
  (UserInterface|Viewport|AddtoViewport _output_get 0))

(event EventUpdatedGameRoundPoints
  (params (Points :type Integer))
  (Variables|/Game/AtomicThreat/Blueprints/UI/WBP_GameRound.WBP_GameRound_C|SetScore (Variables|Default|GetGameRoundWidget) Points))

(event EventCreateNextRoundWidget
  (params (TotalPoints :type Integer) (CityPoints :type Integer) (AmmoPoints :type Integer))
  (bind _returnvalue (UserInterface|CreateWidget "/Game/AtomicThreat/Blueprints/UI/WBP_NextRound.WBP_NextRound_C" 0 TotalPoints CityPoints AmmoPoints))
  (bind _output_get (Variables|Default|SetNexRoundWidget _returnvalue))
  (UserInterface|Viewport|AddtoViewport _output_get 0))

(event EventRemoveGameRoundWidget
  (Widget|RemovefromParent (Variables|Default|GetGameRoundWidget)))

(fn ConstructionScript)