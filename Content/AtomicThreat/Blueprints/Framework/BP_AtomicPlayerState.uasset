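; Player state for AtomicThreat that tracks a player's score.
; The AddPoints event scales incoming points by ScoreBonus, adds them to PlayerScore, then passes the new total to CurrentAtomicPlayer through UpdatedGameRoundPointsMessage.
; GetPoints returns the current total, and a leftover debug print of the score is disconnected.
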(event EventAddPoints
  (params (Points :type Integer))
  (bind _output_get (Variables|Default|SetPlayerScore (+ (* Points (Variables|Default|GetScoreBonus)) (Variables|Default|GetPlayerScore))))
  (Class|BPIAtomicPlayer|UpdatedGameRoundPoints(Message) (Variables|Default|GetCurrentAtomicPlayer) _output_get))

(fn ConstructionScript)

(fn GetPoints
  (return (Variables|Default|GetPlayerScore)))