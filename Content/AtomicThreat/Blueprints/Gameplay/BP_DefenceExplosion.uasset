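; BP_DefenceExplosion is a timed explosion that destroys point-bearing actors it touches and awards their points to the player.
; A timeline, rate-scaled by Duration, drives a sphere trace radius from Size each update, then destroys the explosion when finished.
; Each single-hit trace reads points from the hit component's owner through BPI_Points, adds them to the RocketPlayerController's PlayerState, then destroys that owner.
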(event Custom|TraceExp
  (params (Size :type Float%20%28single-precision%29))
  (bind _returnvalue (Transformation|GetActorLocation))
  (bind _rocketplayercontroller (Variables|Default|GetRocketPlayerController))
  (bind _playerstate (Variables|/Script/Engine.Controller|GetPlayerState _rocketplayercontroller))
  (bind (_outhit _returnvalue_2) (Collision|SphereTraceByChannel _returnvalue _returnvalue Size "TraceTypeQuery4" false 0 "ForDuration" true "(R=1.000000,G=0.000000,B=0.000000,A=1.000000)" "(R=0.000000,G=1.000000,B=0.000000,A=1.000000)" 0.0))
  (if _returnvalue_2
    (if (Utilities|DoesObjectImplementInterface (Components|GetOwner (.HitComponent (Collision|BreakHitResult _outhit))) "/Game/AtomicThreat/Blueprints/Common/BPI_Points.BPI_Points_C")
      (bind _points (Class|BPIPoints|GetPoints(Message) (Components|GetOwner (.HitComponent (Collision|BreakHitResult _outhit)))))
      (if (Utilities|DoesObjectImplementInterface _playerstate "/Game/AtomicThreat/Blueprints/Common/BPI_Points.BPI_Points_C")
        (Class|BPIPoints|AddPoints(Message) _playerstate _points)
        (Actor|DestroyActor (Components|GetOwner (.HitComponent (Collision|BreakHitResult _outhit))))))))

(event EventBeginPlay
  (Components|Timeline|SetPlayRate (Variables|Default|GetExplosionTimeLine) (/ (Components|Animation|GetPlayRate (Variables|Default|GetExplosionTimeLine)) (Variables|Default|GetDuration)))
  (bind _explosionsize (Timeline|ExplosionTimeLine Play)
    (:Update
      (CallFunction|TraceExp (* (Variables|Default|GetSize) _explosionsize)))
    (:Finished
      (Actor|DestroyActor))))

(fn ConstructionScript)