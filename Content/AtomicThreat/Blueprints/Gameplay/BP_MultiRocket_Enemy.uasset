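; BP_MultiRocket_Enemy is an enemy rocket that splits into several rockets after a short, randomized delay.
; The construction script randomizes DecayTime, which drives a one-shot timer from BeginPlay to Decay.
; Decay spawns a random number of RocketType actors at its location with random targets, boosts their parameters, then destroys itself.
; SetTargetsArray supplies the target list, and a separately evaluated random pick removes an entry after each spawn.
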(event Custom|Decay
  (bind _targets (Variables|Default|GetTargets))
  (bind (_outitem _outindex) (Utilities|Array|Random _targets))
  (for _index (range 0 (Math|Random|RandomIntegerinRange 2 4))
    (bind _returnvalue (Game|SpawnActorfromClass (Variables|Default|GetRocketType) (Math|Transform|MakeTransform (Transformation|GetActorLocation) "90.000000, 0, 0" "1,1,1") "Undefined" 0 _outitem 0))
    (Default|IncreaseDefaultRocketParams _returnvalue (Variables|Default|GetIncrease%20Value))
    (Utilities|Array|RemoveIndex _targets _outindex))
  (CallFunction|DestroyRocket))

(event EventBeginPlay
  (|CallParentFunction)
  (Utilities|Time|SetTimerbyEvent (delegate Custom|Decay) (Variables|Default|GetDecayTime)))

(event Collision|EventActorBeginOverlap
  (params (OtherActor :type Actor%20Object%20Reference)))

(event EventTick
  (params (DeltaSeconds :type Float%20%28single-precision%29))
  (|CallParentFunction DeltaSeconds) ; This node is disabled and will not be called.\nDrag off pins to build functionality.
)

(event EventSetTargetsArray
  (params (Targets :type Array%20of%20Vectors))
  (Variables|Default|SetTargets Targets))

(fn ConstructionScript
  (|CallParentFunction)
  (Variables|Default|SetDecayTime (Math|Random|RandomFloatinRange 3.0 5.0)))