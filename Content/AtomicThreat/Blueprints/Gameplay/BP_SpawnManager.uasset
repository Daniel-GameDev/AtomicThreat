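; Spawn manager that launches each round's enemy rockets from upper, left and right launcher grids, registering itself with the game mode.
; At round start it caches target-grid positions, pulls rocket count and types from difficulty data, and assigns random spawn times.
; A looping timer launches random rockets as times come due and broadcasts the remaining count.
; Side-launch rockets aim at the same index on the opposite grid; others fire from above at random targets.
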(event Custom|SpawnerStartRound
  (Utilities|FlowControl|Sequence
    (:then_0
      (for _array_element (Variables|Default|GetTargetGridRef)
        (Utilities|Array|Add (Variables|Default|GetTargetVectors) (Transformation|GetWorldLocation (Variables|/Script/Engine.Actor|GetRootComponent _array_element)))))
    (:then_1
      (bind (_rocketsnum _difficultyincrement _rocketsstructurearray) (CallFunction|GetDifficultyDataFunction (Variables|Default|GetRound)))
      (Variables|Default|SetRocketsNum _rocketsnum)
      (Variables|Default|SetDifficultyIncrement _difficultyincrement)
      (Variables|Default|SetRocketsToSpawn _rocketsstructurearray)
      (for _index (range 1 (Variables|Default|GetRocketsNum))
        (Utilities|Array|Add (Variables|Default|GetAssignedTime) (Math|Random|RandomFloatinRange (Variables|Default|GetSpawnFrequencyMin) (Variables|Default|GetSpawnFrequencyMax))))
      (bind _returnvalue (Utilities|Time|SetTimerbyEvent (delegate Custom|BeginSpawn) (Variables|Default|GetTimerFrequency) true))
      (Variables|Default|SetTimerRef _returnvalue))))

(event Custom|UpdateDifficulty
  (params (Round :type Integer))
  (Variables|Default|SetRound Round))

(event Custom|BeginSpawn
  (bind _rocketspawned (CallFunction|SpawnEnemyRockets))
  (if _rocketspawned
    (bind _result (Math|Integer|DecrementInt (Variables|Default|GetRocketsNum))
      (:%20%20
        (Default|CallRocketSpawned _result)
        (if (== (Utilities|Array|Length (Variables|Default|GetAssignedTime)) 0)
          (Utilities|Time|ClearandInvalidateTimerbyHandle (Variables|Default|GetTimerRef)))))))

(event EventBeginPlay
  (Utilities|FlowControl|Sequence
    (:then_0
      (bind _gridref (Default|CreateGrid2 (Variables|Default|GetUpperEnemyGrid) true (Utilities|Array|MakeArray 0)))
      (Variables|Default|SetUpperEnemyGridElements _gridref))
    (:then_1
      (bind _gridref_2 (Default|CreateGrid2 (Variables|Default|GetRightSideEnemyGrid) true (Utilities|Array|MakeArray 0)))
      (Variables|Default|SetRightSideEnemyGridElements _gridref_2))
    (:then_2
      (bind _gridref_3 (Default|CreateGrid2 (Variables|Default|GetLeftSideEnemyGrid) true (Utilities|Array|MakeArray 0)))
      (Variables|Default|SetLeftSideEnemyGridElements _gridref_3))
    (:then_3
      ;[1 1 1] try to move this to GameMode by C++
      (bind _asbp_atomic_game_mode (Utilities|Casting|CastToBP_AtomicGameMode (Game|GetGameMode)))
      (Variables|/Game/AtomicThreat/Blueprints/Framework/BP_AtomicGameMode.BP_AtomicGameMode_C|SetSpawnManager _asbp_atomic_game_mode self))))

(fn ConstructionScript)

(fn SpawnEnemyRockets
  (bind _leftsideenemygridelements (Variables|Default|GetLeftSideEnemyGridElements))
  (bind _rightsideenemygridelements (Variables|Default|GetRightSideEnemyGridElements))
  (for (_array_element _array_index) (Variables|Default|GetAssignedTime)
    (if (<= _array_element (Variables|Default|GetTimerValue))
      (Utilities|Array|RemoveIndex (Variables|Default|GetAssignedTime) _array_index)
      (bind (_empty _rocketclass) (CallFunction|GetRandomRocket))
      (if (not _empty)
        (LocalVariables|SetLocal_RocketClass _rocketclass)
        (if (Math|Boolean|Equal(Boolean) (.SideLaunch (Utilities|GetClassDefaults _rocketclass)) true)
          (switch Utilities|FlowControl|Switch|SwitchonESides (Utilities|Enum|ByteToEnumESides (Math|Conversions|ToByte(Integer) (Math|Random|RandomIntegerinRange 0 (- (|GetNumEnumEntries) 1))))
            (:NewEnumerator0
              (bind _output_get (LocalVariables|SetLocal_RandomIndex (.OutIndex (Utilities|Array|Random _rightsideenemygridelements))))
              (bind _asbp_enemy_launcher_grid_element (Utilities|Casting|CastToBP_EnemyLauncher_GridElement (Utilities|Array|Get(acopy) _rightsideenemygridelements _output_get)))
              (Default|LaunchRocket _asbp_enemy_launcher_grid_element (LocalVariables|GetLocal_RocketClass) (Variables|Default|GetDifficultyIncrement) (Transformation|GetWorldLocation (Variables|/Script/Engine.Actor|GetRootComponent (Utilities|Array|Get(acopy) (Variables|Default|GetLeftSideEnemyGridElements) (LocalVariables|GetLocal_RandomIndex)))) (Variables|Default|GetTargetVectors))
              (return true))
            (:NewEnumerator1
              (bind _output_get_2 (LocalVariables|SetLocal_RandomIndex (.OutIndex (Utilities|Array|Random _leftsideenemygridelements))))
              (bind _asbp_enemy_launcher_grid_element_2 (Utilities|Casting|CastToBP_EnemyLauncher_GridElement (Utilities|Array|Get(acopy) _leftsideenemygridelements _output_get_2)))
              (Default|LaunchRocket _asbp_enemy_launcher_grid_element_2 (LocalVariables|GetLocal_RocketClass) (Variables|Default|GetDifficultyIncrement) (Transformation|GetWorldLocation (Variables|/Script/Engine.Actor|GetRootComponent (Utilities|Array|Get(acopy) (Variables|Default|GetRightSideEnemyGridElements) (LocalVariables|GetLocal_RandomIndex)))) (Variables|Default|GetTargetVectors))
              (return true)))
          (else
            (bind _asbp_enemy_launcher_grid_element_3 (Utilities|Casting|CastToBP_EnemyLauncher_GridElement (.OutItem (Utilities|Array|Random (Variables|Default|GetUpperEnemyGridElements)))))
            (Default|LaunchRocket _asbp_enemy_launcher_grid_element_3 (LocalVariables|GetLocal_RocketClass) (Variables|Default|GetDifficultyIncrement) (.OutItem (Utilities|Array|Random (Variables|Default|GetTargetVectors))) (Variables|Default|GetTargetVectors))
            (return true))))))
  (Variables|Default|SetTimerValue (Math|Float|Clamp(Float) (+ (Variables|Default|GetTimerValue) 0.5) (Variables|Default|GetSpawnFrequencyMin) (Variables|Default|GetSpawnFrequencyMax)))
  (return false))

(fn GetRandomRocket
  (bind _rocketstospawn (Variables|Default|GetRocketsToSpawn))
  (for (_ _array_index) _rocketstospawn
    (if (!= _array_index -1)
      (bind _output_get (LocalVariables|SetLocal_Index (.OutIndex (Utilities|Array|Random _rocketstospawn))))
      (bind _result (Math|Integer|DecrementInt (.num (Utilities|Array|Get(acopy) (Variables|Default|GetRocketsToSpawn) _output_get)))
        (:%20%20
          (LocalVariables|SetLocal_RocketClass (.rockettype (Utilities|Array|Get(acopy) (Variables|Default|GetRocketsToSpawn) _output_get)))
          (if (== _result 0)
            (Utilities|Array|RemoveIndex (Variables|Default|GetRocketsToSpawn) (LocalVariables|GetLocal_Index))
            (return false (LocalVariables|GetLocal_RocketClass))
            (else
              (return false (LocalVariables|GetLocal_RocketClass))))))
      (else
        (return true 0)))))

(fn CreateTargetGird
  (params (Use%20Default%20Grid :type Boolean) (GridElements :type Array%20of%20BP%20Grid%20Element%20Base%20Class%20References))
  (Default|ClearGrid2 (Variables|Default|GetTargetGrid))
  (bind _gridref (Default|CreateGrid2 (Variables|Default|GetTargetGrid) Use%20Default%20Grid GridElements))
  (bind _output_get (Variables|Default|SetTargetGridRef _gridref))
  (return _output_get))