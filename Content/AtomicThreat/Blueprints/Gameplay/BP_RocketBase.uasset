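; BP_RocketBase is a base homing rocket that flies toward a Target location and destroys itself on arrival.
; On BeginPlay it spawns a BP_Target marker there and sets its root as the ProjectileMovement homing target.
; Tick rolls RocketForward, optionally draws debug lines for the trail and start-to-target path, and checks proximity to Target.
; Arrival destroys both the marker and the rocket, with no damage logic.
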(event Custom|TargetHit
  (CallFunction|DestroyRocket))

(event Custom|DestroyRocket
  (Actor|DestroyActor (Components|GetOwner (Variables|Default|GetTargetSceneRoot)))
  (Actor|DestroyActor))

(event Custom|DrawRocketDebug
  (bind _returnvalue (Transformation|GetActorLocation))
  (Rendering|Debug|DrawDebugLine (Variables|Default|GetPreviousPoint) _returnvalue "(R=1.000000,G=0.003080,B=0.000000,A=1.000000)" 1.5 2e+01)
  (Variables|Default|SetPreviousPoint _returnvalue)
  (Rendering|Debug|DrawDebugLine (Variables|Default|GetStartPoint) (Variables|Default|GetTarget) "(R=0.000000,G=0.018481,B=1.000000,A=1.000000)" 5.0 5e+01))

(event EventBeginPlay
  (bind _returnvalue (Transformation|GetActorLocation))
  (Utilities|FlowControl|Sequence
    (:then_0
      (Variables|Default|SetStartPoint _returnvalue)
      (Variables|Default|SetPreviousPoint _returnvalue))
    (:then_1
      (bind _returnvalue_2 (Game|SpawnActorfromClass "/Game/AtomicThreat/Blueprints/Gameplay/BP_Target.BP_Target_C" (Math|Transform|MakeTransform (Variables|Default|GetTarget) "0, 0, 0" "1,1,1") "Undefined" 0 0))
      (bind _output_get (Variables|Default|SetTargetSceneRoot (Variables|/Game/AtomicThreat/Blueprints/Gameplay/BP_Target.BP_Target_C|GetDefaultSceneRoot _returnvalue_2)))
      (Variables|/Script/Engine.ProjectileMovementComponent|SetHomingTargetComponent (Variables|Default|GetProjectileMovement) _output_get))))

(event EventTick
  (params (DeltaSeconds :type Float%20%28single-precision%29))
  (CallFunction|Rotate DeltaSeconds)
  (if (Variables|Default|GetDrawDebugLines)
    (CallFunction|DrawRocketDebug))
  (if (Math|Vector|Equal(Vector) (Transformation|GetActorLocation) (Variables|Default|GetTarget) 4e+02)
    (CallFunction|TargetHit)))

(fn ConstructionScript)

(fn Rotate
  (params (Tick :type Float%20%28single-precision%29))
  (Transformation|SetRelativeRotation (Variables|Default|GetRocketForward) (Math|Rotator|MakeRotator (+ (* Tick (Variables|Default|GetRotationSpeed)) (.roll (Variables|/Script/Engine.SceneComponent|GetRelativeRotation (Variables|Default|GetRocketForward)))) 0.0 0.0) false false))