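; BP_MapGrid is an actor that builds a line of map grid elements at BeginPlay.
; For each class in the GridElements map, it adds an attachment point component one GridSpacing further along Y, then spawns and attaches that element.
; Spawned BP_GridElementBase actors receive their iteration index.
; The construction script is empty, with an unconnected loop for placing hex meshes left in it.
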(event Custom|CreateGrid
  (bind _values (Utilities|Map|Values (Variables|Default|GetGridElements)))
  (for (_array_element _array_index) _values
    (bind _returnvalue (Game|AddComponentbyClass "/Game/AtomicThreat/Blueprints/Gameplay/BP_GridAttachmentPointComponent.BP_GridAttachmentPointComponent_C" false (Math|Transform|MakeTransform (Math|Vector|MakeVector (.X (Math|Vector|BreakVector (Variables|Default|GetComponentLocation))) (+ (.Y (Math|Vector|BreakVector (Variables|Default|GetComponentLocation))) (Variables|Default|GetGridSpacing)) (.Z (Math|Vector|BreakVector (Variables|Default|GetComponentLocation)))) "0, 0, 0" "1,1,1")))
    (bind _output_get (Variables|Default|SetComponentLocation (Variables|/Script/Engine.SceneComponent|GetRelativeLocation _returnvalue)))
    (bind _returnvalue_2 (Game|SpawnActorfromClass _array_element (Math|Transform|MakeTransform _output_get "0, 0, 0" "1,1,1") "Undefined" 0 0))
    (Transformation|AttachComponentToComponent _returnvalue_2 _returnvalue "None" "KeepRelative" "KeepRelative" "KeepRelative" true)
    (bind _asbp_grid_element_base (Utilities|Casting|CastToBP_GridElementBase _returnvalue_2))
    (Variables|/Game/AtomicThreat/Blueprints/Gameplay/BP_GridElementBase.BP_GridElementBase_C|SetIndex _asbp_grid_element_base _array_index)))

(event EventBeginPlay
  (CallFunction|CreateGrid))

(fn ConstructionScript)