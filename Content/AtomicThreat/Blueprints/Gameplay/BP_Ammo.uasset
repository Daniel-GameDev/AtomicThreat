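; BP_Ammo is a visible rocket ammo stock that creates one static mesh component per round of its default ammo size on BeginPlay.
; SetAmmoPosition centers the first rocket on Zero and alternates the rest under Odd and Even anchors, spacing them along Y by child count.
; UseAmmo destroys the last rocket and returns true only when the stock is already empty.
; DetachComponents reparents the side anchors' children to Arrow.
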(event EventBeginPlay
  (for _index (range 1 (Variables|Default|GetDefaultAmmoSize))
    (bind _returnvalue (Game|AddComponentbyClass "/Script/Engine.StaticMeshComponent" false))
    (Components|StaticMesh|SetStaticMesh _returnvalue (Variables|Default|GetRocketMesh))
    (Utilities|Array|Add (Variables|Default|GetRockets) _returnvalue))
  (CallFunction|SetAmmoPosition))

(fn ConstructionScript)

(fn UseAmmo
  (bind _rockets (Variables|Default|GetRockets))
  (bind _rockets_2 (Variables|Default|GetRockets))
  (bind _returnvalue (Utilities|Array|Length _rockets))
  (bind _returnvalue_2 (- _returnvalue 1))
  (if (== (Utilities|Array|Length (Variables|Default|GetRockets)) 0)
    (return true)
    (else
      (Components|DestroyComponent (Utilities|Array|Get(acopy) _rockets_2 _returnvalue_2))
      (Utilities|Array|RemoveIndex _rockets_2 _returnvalue_2)
      (return false))))

(fn SetAmmoPosition
  (bind _even (Variables|Default|GetEven))
  (bind _odd (Variables|Default|GetOdd))
  (for (_array_element _array_index) (Variables|Default|GetRockets)
    (LocalVariables|SetLocal_ArrayElement _array_element)
    (if (== _array_index 0)
      (Transformation|AttachComponentToComponent (LocalVariables|GetLocal_ArrayElement) (Variables|Default|GetZero) "None" "KeepRelative" "KeepRelative" "KeepRelative" false)
      (elif (> (Math|Integer|%(Integer) _array_index 2) 0)
        (Transformation|SetRelativeLocation (LocalVariables|GetLocal_ArrayElement) (Math|Vector|MakeVector 0.0 (.y (* (Variables|/Script/Engine.SceneComponent|GetRelativeLocation _odd) (Class|SceneComponent|GetNumChildrenComponents _odd))) 0.0) false false)
        (Transformation|AttachComponentToComponent (LocalVariables|GetLocal_ArrayElement) (Variables|Default|GetOdd) "None" "KeepRelative" "KeepRelative" "KeepRelative" false)
        (else
          (Transformation|SetRelativeLocation (LocalVariables|GetLocal_ArrayElement) (Math|Vector|MakeVector 0.0 (.y (* (Variables|/Script/Engine.SceneComponent|GetRelativeLocation _even) (Class|SceneComponent|GetNumChildrenComponents _even))) 0.0) false false)
          (Transformation|AttachComponentToComponent (LocalVariables|GetLocal_ArrayElement) (Variables|Default|GetEven) "None" "KeepRelative" "KeepRelative" "KeepRelative" false))))))

(fn DetachComponents
  (for _array_element (Components|GetChildrenComponents (Variables|Default|GetEven) true)
    (Transformation|AttachComponentToComponent _array_element (Variables|Default|GetArrow) "None" "KeepRelative" "KeepRelative" "KeepRelative" false))
  (for _array_element_2 (Components|GetChildrenComponents (Variables|Default|GetOdd) true)
    (Transformation|AttachComponentToComponent _array_element_2 (Variables|Default|GetArrow) "None" "KeepRelative" "KeepRelative" "KeepRelative" false)))