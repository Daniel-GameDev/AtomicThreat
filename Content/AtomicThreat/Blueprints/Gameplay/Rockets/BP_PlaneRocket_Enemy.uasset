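; Enemy plane rocket carrier that releases a rocket of a configurable type after a random delay chosen at construction.
; A one-shot timer spawns the rocket at the RocketHolder with a fixed rotation and a random target, then raises its parameters by the difficulty increment.
; Rockets implementing BPI_MultiRocket also receive the full target array, and only in that case is the holder component destroyed.
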(event Custom|Decay
  (bind _returnvalue (Game|SpawnActorfromClass (Variables|Default|GetRocketType) (Math|Transform|MakeTransform (Transformation|GetWorldLocation (Variables|Default|GetRocketHolder)) "90.000000, 0, 0" "1,1,1") "Undefined" 0 (.OutItem (Utilities|Array|Random (Variables|Default|GetTargets))) 0))
  (Default|IncreaseDefaultRocketParams _returnvalue (Variables|Default|GetDifficultyIncrement))
  (if (Utilities|DoesObjectImplementInterface _returnvalue "/Game/AtomicThreat/Blueprints/Common/BPI_MultiRocket.BPI_MultiRocket_C")
    (Class|BPIMultiRocket|SetTargetsArray(Message) _returnvalue (Variables|Default|GetTargets))
    (Components|DestroyComponent (Variables|Default|GetRocketHolder))))

(event EventBeginPlay
  (|CallParentFunction)
  (Utilities|Time|SetTimerbyEvent (delegate Custom|Decay) (Variables|Default|GetDecayTime)))

(event Collision|EventActorBeginOverlap
  (params (OtherActor :type Actor%20Object%20Reference)))

(event EventTick
  (params (DeltaSeconds :type Float%20%28single-precision%29))
  (|CallParentFunction DeltaSeconds) ; This node is disabled and will not be called.\nDrag off pins to build functionality.
)

(event EventSetTargetsArray
  (params (Targets :type Array%20of%20Vectors))
  (Variables|Default|SetTargets Targets))

(fn ConstructionScript
  (|CallParentFunction)
  (Variables|Default|SetDecayTime (Math|Random|RandomFloatinRange 3.0 5.0)))