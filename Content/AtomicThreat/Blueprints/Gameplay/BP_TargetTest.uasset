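; BP_TargetTest is a test target actor that spins its Scene component.
; Each tick it adds a Roll variable to the component's current relative roll, resetting pitch and yaw to zero.
; The increment is not scaled by delta time, so the spin speed depends on frame rate.
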(event EventBeginPlay
  (|CallParentFunction) ; This node is disabled and will not be called.\nDrag off pins to build functionality.
)

(event Collision|EventActorBeginOverlap
  (params (OtherActor :type Actor%20Object%20Reference))
  (|CallParentFunction OtherActor) ; This node is disabled and will not be called.\nDrag off pins to build functionality.
)

(event EventTick
  (params (DeltaSeconds :type Float%20%28single-precision%29))
  (|CallParentFunction DeltaSeconds)
  (Transformation|SetRelativeRotation (Variables|Default|GetScene) (Math|Rotator|MakeRotator (+ (.roll (Variables|/Script/Engine.SceneComponent|GetRelativeRotation (Variables|Default|GetScene))) (Variables|Default|GetRoll)) 0.0 0.0) false false))

(fn ConstructionScript
  (|CallParentFunction))