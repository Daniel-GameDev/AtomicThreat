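; Showcase variant of the East Su-25 bomber that exposes the aircraft's moving parts and appearance to generic checkbox and slider controls.
; Each control event forwards to setters for damage display, control surfaces, lights, canopy, air brake, landing gear retraction and suspension, driving left and right sides together.
; Any gear retraction locks wheel suspension through CanSuspendWheels; full extension unlocks it and resets suspension to zero.
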(event EventBeginPlay
  (|CallParentFunction) ; This node is disabled and will not be called.\nDrag off pins to build functionality.
)

(event Collision|EventActorBeginOverlap
  (params (OtherActor :type Actor%20Object%20Reference))
  (|CallParentFunction OtherActor) ; This node is disabled and will not be called.\nDrag off pins to build functionality.
)

(event EventSetSliderVariable2
  (params (NewValue :type Float%20%28single-precision%29))
  (CallFunction|SetAileronL NewValue)
  (CallFunction|SetAileronR NewValue))

(event EventSetSliderVariable3
  (params (NewValue :type Float%20%28single-precision%29))
  (CallFunction|SetFlapsL NewValue)
  (CallFunction|SetFlapsR NewValue))

(event EventSetSliderVariable4
  (params (NewValue :type Float%20%28single-precision%29))
  (CallFunction|SetLightsEmissivity NewValue))

(event EventSetTwinSliderVariable0
  (params (bFirstSlider? :type Boolean) (NewFirstValue :type Float%20%28single-precision%29) (NewSecondValue :type Float%20%28single-precision%29))
  (CallFunction|RetractFrontWheel NewFirstValue)
  (CallFunction|RetractRearRWheel NewSecondValue)
  (CallFunction|RetractRearLWheel NewSecondValue)
  (if (or (> NewFirstValue 0.0) (> NewSecondValue 0.0))
    (Variables|Default|SetcanSuspendWheels false)
    (else
      (Variables|Default|SetcanSuspendWheels true)
      (CallFunction|SetFrontWheelSuspension 0.0)
      (CallFunction|SetRearWheelLSuspension 0.0)
      (CallFunction|SetRearWheelRSuspension 0.0))))

(event EventTick
  (params (DeltaSeconds :type Float%20%28single-precision%29))
  (|CallParentFunction DeltaSeconds) ; This node is disabled and will not be called.\nDrag off pins to build functionality.
)

(event EventSetCheckboxVariable0
  (params (NewState :type Boolean))
  (CallFunction|SetShowDamaged NewState))

(event EventSetTwinSliderVariable1
  (params (bFirstSlider? :type Boolean) (NewFirstValue :type Float%20%28single-precision%29) (NewSecondValue :type Float%20%28single-precision%29))
  (CallFunction|SetCanopyOpen NewFirstValue)
  (CallFunction|SetAirBrake NewSecondValue))

(event EventSetTwinSliderVariable2
  (params (bFirstSlider? :type Boolean) (NewFirstValue :type Float%20%28single-precision%29) (NewSecondValue :type Float%20%28single-precision%29))
  ;[1 0.4792 0.4792] Wheels must be Fully Extended
  (if (Variables|Default|GetcanSuspendWheels)
    (CallFunction|SetFrontWheelSuspension NewFirstValue)
    (CallFunction|SetRearWheelLSuspension NewSecondValue)
    (CallFunction|SetRearWheelRSuspension NewSecondValue)))

(event EventSetSliderVariable0
  (params (NewValue :type Float%20%28single-precision%29))
  (CallFunction|SetRudder NewValue))

(event EventSetSliderVariable1
  (params (NewValue :type Float%20%28single-precision%29))
  (CallFunction|SetStabilizersL NewValue)
  (CallFunction|SetStabilizersR NewValue))

(fn ConstructionScript
  (|CallParentFunction))